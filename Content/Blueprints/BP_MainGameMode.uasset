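; BP_MainGameMode is the game mode that decides the outcome when the game ends.
; Its CheckWinLoseCondition event acts only once IsGameOver is set, then pauses the game and clears all widgets.
; It compares CurrentScore against MinimumRequiredScore and calls WonGame or LostGame, each adding its matching result widget to the viewport.
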(event Custom|CheckWinLoseCondition
  (if (Variables|Default|GetIsGameOver)
    (Game|SetGamePaused true)
    (Viewport|RemoveAllWidgets)
    (if (>= (Variables|Default|GetCurrentScore) (Variables|Default|GetMinimumRequiredScore))
      (CallFunction|WonGame)
      (else
        (CallFunction|LostGame)))))

(event EventBeginPlay
  (|CallParentFunction))

(fn ConstructionScript)

(fn WonGame
  (bind _returnvalue (UserInterface|CreateWidget "/Game/Blueprints/UserWidgets/BPW_GameWon.BPW_GameWon_C" (Game|GetPlayerController 0)))
  (UserInterface|Viewport|AddtoViewport _returnvalue 0))

(fn LostGame
  (bind _returnvalue (UserInterface|CreateWidget "/Game/Blueprints/UserWidgets/BPW_GameLost.BPW_GameLost_C" (Game|GetPlayerController 0)))
  (UserInterface|Viewport|AddtoViewport _returnvalue 0))