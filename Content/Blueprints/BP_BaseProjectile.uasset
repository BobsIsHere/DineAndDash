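; BP_BaseProjectile is a base projectile that deals damage on impact, then destroys itself.
; Both hit and overlap events on its collision component feed ProcessCollision, which skips invalid actors and those carrying IgnoreTag.
; It sends DoDamage through the damageable interface to the actor and each implementing component, playing an impact sound each time and rechecking actor validity as it goes.
; An impact effect spawns before destruction, even when the target is not damageable.
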(event OnComponentHit(Colllision)
  (params (HitComponent :type Primitive%20Component%20Object%20Reference) (OtherActor :type Actor%20Object%20Reference) (OtherComp :type Primitive%20Component%20Object%20Reference) (NormalImpulse :type Vector :default "0, 0, 0") (Hit :type Hit%20Result%20Structure%20%28by%20ref%29))
  (CallFunction|ProcessCollision OtherActor))

(event OnComponentBeginOverlap(Colllision)
  (params (OverlappedComponent :type Primitive%20Component%20Object%20Reference) (OtherActor :type Actor%20Object%20Reference) (OtherComp :type Primitive%20Component%20Object%20Reference) (OtherBodyIndex :type Integer) (bFromSweep :type Boolean) (SweepResult :type Hit%20Result%20Structure%20%28by%20ref%29))
  (CallFunction|ProcessCollision OtherActor))

(event EventBeginPlay)

(event Collision|EventActorBeginOverlap
  (params (OtherActor :type Actor%20Object%20Reference)))

(event EventTick
  (params (DeltaSeconds :type Float%20%28single-precision%29)))

(fn ConstructionScript)

(fn ProcessCollision
  (params (OtherActor :type Actor%20Object%20Reference))
  (bind _returnvalue (Class|Actor|GetComponentsbyInterface OtherActor "/Script/Unreal101.DamageableInterface"))
  (bind _colllision (Variables|Default|GetColllision))
  ;[1 1 1] Check if we actually hit actor
  (Utilities|IsValid OtherActor
    (:Is%20Valid
      ;[1 1 1] Check if target doesn't have matching ignore tag
      (if (not (Actor|ActorHasTag OtherActor (Variables|Default|GetIgnoreTag)))
        (Utilities|FlowControl|Sequence
          (:then_0
            ;[1 1 1] BPI_Damagable on hit actor
            (if (Utilities|DoesObjectImplementInterface OtherActor "/Script/Unreal101.DamageableInterface")
              (Class|DamageableInterface|DoDamage(Message) OtherActor (Variables|Default|GetDamageAmount))
              (Audio|SpawnSoundAttached "/Game/Audio/234082__211redman112__lasgun-impact.234082__211redman112__lasgun-impact" (Variables|Default|GetColllision) "None" "0, 0, 0" "0, 0, 0" "KeepRelativeOffset" false 1.0 1.0 0.0 0 0)))
          (:then_1
            ;[1 1 1] Get all component that implement the BPI_Damagable interface & DoDagame
            (Utilities|IsValid OtherActor
              (:Is%20Valid
                (bind _index (Utilities|FlowControl|ForLoopwithBreak 0 (- (Utilities|Array|Length _returnvalue) 1) :!label _label)
                  (:LoopBody
                    (Class|DamageableInterface|DoDamage(Message) (Utilities|Array|Get(acopy) _returnvalue _index) (Variables|Default|GetDamageAmount))
                    (Audio|SpawnSoundAttached "/Game/Audio/234082__211redman112__lasgun-impact.234082__211redman112__lasgun-impact" (Variables|Default|GetColllision) "None" "0, 0, 0" "0, 0, 0" "KeepRelativeOffset" false 1.0 1.0 0.0 0 0)
                    (Utilities|IsValid OtherActor
                      (:Is%20Not%20Valid
                        (goto _label Break))))))))
          (:then_2
            (Niagara|SpawnSystematLocation "/Game/Particles/FXS_ProjectileImpact.FXS_ProjectileImpact" (Transformation|GetWorldLocation _colllision) (Transformation|GetWorldRotation _colllision))
            ;[1 1 1] Destroy!
            (Actor|DestroyActor)))))))