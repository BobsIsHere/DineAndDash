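; BP_MyGameMode is the game mode that drives customer spawning, keeps the score and decides the win or lose result.
; On BeginPlay it starts a looping timer on every BP_CustomerSpawner that calls Spawn at a configurable per-spawner rate.
; IncrementScore adds to the current score.
; CheckWinLoseCondition compares it to the required minimum once the game is over, and the outcome only prints a message.
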(event Custom|IncrementScore
  (params (ScoreAmount :type Integer))
  ;[1 1 1] Increment Score
  (Variables|Score|SetCurrentScore (+ ScoreAmount (Variables|Score|GetCurrentScore))))

(event Custom|CheckWinLoseCondition
  (if (Variables|Game|GetIsGameOver)
    (if (>= (Variables|Score|GetCurrentScore) (Variables|Score|GetMinimumRequiredScore))
      (CallFunction|WonGame)
      (else
        (CallFunction|LostGame)))))

(event EventBeginPlay
  (bind _outactors (Actor|GetAllActorsOfClass "/Game/Blueprints/BP_CustomerSpawner.BP_CustomerSpawner_C"))
  (bind _output_get (Variables|CustomerSpawns|SetEnemySpawners _outactors))
  (for _array_element _output_get
    (Utilities|Time|SetTimerbyFunctionName _array_element "Spawn" (/ 1.0 (Variables|CustomerSpawns|GetCustomerPerSecondPerSpawner)) true)))

(event EventTick
  (params (DeltaSeconds :type Float%20%28single-precision%29)))

(fn ConstructionScript)

(fn WonGame
  (Development|PrintString "WON :D"))

(fn LostGame
  (Development|PrintString "LOST :("))