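; Player controller that runs the paused main menu and game HUD flow, plus player movement, aiming and interaction.
; Enhanced Input drives movement and stick aim, while cursor traces steer a mouse target marker; movement direction can take over after an aim-idle delay.
; Interact triggers nearby cached BP_Interactables; occupied tables check the character's salt, cheese or herb stock.
; Stocked tables open a timed condiment minigame widget and are freed immediately.
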(event Custom|GameStart
  (Variables|Default|SetbShowMouseCursor false)
  (Game|SetGamePaused false)
  (Widget|RemovefromParent (stale EventBeginPlay _returnvalue_2))
  ;[1 1 1] Setup HUD
  (bind _returnvalue (UserInterface|CreateWidget "/Game/Blueprints/BPW_GameHud.BPW_GameHud_C" self))
  (UserInterface|Viewport|AddtoViewport _returnvalue 0))

(event Custom|StartSaltGameEvent
  ;[1 1 1] Mini Game Events
  (bind _returnvalue (UserInterface|CreateWidget "/Game/Blueprints/BPW_SaltMiniGame.BPW_SaltMiniGame_C" self))
  (UserInterface|Viewport|AddtoViewport _returnvalue 0)
  (Variables|MiniGames|SetSaltMiniGameHUD _returnvalue)
  (Utilities|FlowControl|Delay (Variables|MiniGames|GetMiniGameDuration))
  (CallFunction|EndMiniGame (Variables|MiniGames|GetSaltMiniGameHUD))
  (Development|PrintString "Done Salt"))

(event Custom|StartCheeseGameEvent
  ;[1 1 1] Mini Game Events
  (bind _returnvalue (UserInterface|CreateWidget "/Game/Blueprints/BPW_CheeseMiniGame.BPW_CheeseMiniGame_C" self))
  (UserInterface|Viewport|AddtoViewport _returnvalue 0)
  (Variables|MiniGames|SetCheeseMiniGameHUD _returnvalue)
  (Utilities|FlowControl|Delay (Variables|MiniGames|GetMiniGameDuration))
  (CallFunction|EndMiniGame (Variables|MiniGames|GetCheeseMiniGameHUD))
  (Development|PrintString "Done Cheese"))

(event Custom|StartHerbsGameEvent
  ;[1 1 1] Mini Game Events
  (bind _returnvalue (UserInterface|CreateWidget "/Game/Blueprints/BPW_HerbsMiniGame.BPW_HerbsMiniGame_C" self))
  (UserInterface|Viewport|AddtoViewport _returnvalue 0)
  (Variables|MiniGames|SetHerbsMiniGameHUD _returnvalue)
  (Utilities|FlowControl|Delay (Variables|MiniGames|GetMiniGameDuration))
  (CallFunction|EndMiniGame (Variables|MiniGames|GetHerbsMiniGameHUD))
  (Development|PrintString "Done Herbs"))

(event Input|EnhancedActionEvents|EnhancedInputActionIA_PlayerAim
  (params (ActionValue :type Vector%202D%20Structure) (ElapsedSeconds :type Float%20%28double-precision%29) (TriggeredSeconds :type Float%20%28double-precision%29) (InputAction :type Input%20Action%20Object%20Reference :default "/Game/Input/Actions/IA_PlayerAim.IA_PlayerAim"))
  (bind _returnvalue (Math|Vector|MakeVector (.y ActionValue) (.x ActionValue) 0.0))
  ;[0.08235 0.1059 1] Gamepad Aiming
  ;;[1 0.4179 0] Mouse Aim Detection
  (Variables|MouseAiming|SetUseMouseAim (> (Math|Vector|VectorLengthSquared _returnvalue) 0.2))
  (bind _currentmouseaimtarget (Variables|MouseAiming|GetCurrentMouseAimTarget)
    (:then
      (Rendering|SetActorHiddenInGame _currentmouseaimtarget true))
    (:else
      _))
  (Pawn|SetControlRotation (Math|Conversions|RotationFromXVector _returnvalue))
  (Variables|MouseAiming|SetLastAimInputTime (Utilities|Time|GetTimeSeconds)))

(event Input|EnhancedActionEvents|EnhancedInputActionIA_PlayerInteraction
  (params (ActionValue :type Boolean) (ElapsedSeconds :type Float%20%28double-precision%29) (TriggeredSeconds :type Float%20%28double-precision%29) (InputAction :type Input%20Action%20Object%20Reference :default "/Game/Input/Actions/IA_PlayerInteraction.IA_PlayerInteraction"))
  ;[0.08235 0.1059 1] Interactable Input
  (for _array_element (Variables|Interactables|GetInteractables)
    (if (Variables|/Game/Blueprints/BP_Interactable.BP_Interactable_C|GetIsPlayerNearby _array_element)
      (Default|Interact _array_element)
      (bind _asbpi_table (Utilities|Casting|CastToBPI_Table _array_element))
      (if (Variables|/Game/Blueprints/BPI_Table.BPI_Table_C|GetIsTableOccupied _asbpi_table)
        (switch Utilities|FlowControl|Switch|SwitchonECondimentType (Variables|/Game/Blueprints/BPI_Table.BPI_Table_C|GetCondimentType _asbpi_table)
          (:NewEnumerator0
            (bind _asbp_player_character (Utilities|Casting|CastToBP_PlayerCharacter (Game|GetPlayerCharacter 0)))
            (if (== (Variables|/Game/Blueprints/BP_PlayerCharacter.BP_PlayerCharacter_C|GetSaltAmount _asbp_player_character) 0)
              (Development|PrintString "REFILL SALT FIRST!")
              (else
                (CallFunction|StartSaltGameEvent)
                (Variables|/Game/Blueprints/BPI_Table.BPI_Table_C|SetIsTableOccupied _asbpi_table false))))
          (:NewEnumerator1
            (bind _asbp_player_character_2 (Utilities|Casting|CastToBP_PlayerCharacter (Game|GetPlayerCharacter 0)))
            (if (== (Variables|/Game/Blueprints/BP_PlayerCharacter.BP_PlayerCharacter_C|GetCheeseAmount _asbp_player_character_2) 0)
              (Development|PrintString "REFILL CHEESE FIRST!")
              (else
                (CallFunction|StartCheeseGameEvent)
                (Variables|/Game/Blueprints/BPI_Table.BPI_Table_C|SetIsTableOccupied _asbpi_table false))))
          (:NewEnumerator2
            (bind _asbp_player_character_3 (Utilities|Casting|CastToBP_PlayerCharacter (Game|GetPlayerCharacter 0)))
            (if (== (Variables|/Game/Blueprints/BP_PlayerCharacter.BP_PlayerCharacter_C|GetHerbAmount _asbp_player_character_3) 0)
              (Development|PrintString "REFILL HERBS FIRST!")
              (else
                (CallFunction|StartHerbsGameEvent)
                (Variables|/Game/Blueprints/BPI_Table.BPI_Table_C|SetIsTableOccupied _asbpi_table false)))))))))

(event Input|EnhancedActionEvents|EnhancedInputActionIA_PlayerMovement
  (params (ActionValue :type Vector%202D%20Structure) (ElapsedSeconds :type Float%20%28double-precision%29) (TriggeredSeconds :type Float%20%28double-precision%29) (InputAction :type Input%20Action%20Object%20Reference :default "/Game/Input/Actions/IA_PlayerMovement.IA_PlayerMovement"))
  (bind _returnvalue (Pawn|GetControlledPawn))
  (bind _returnvalue_2 (Class|Pawn|GetLastMovementInputVector _returnvalue))
  (bind _returnvalue_3 (Math|Conversions|RotationFromXVector _returnvalue_2))
  ;[0.08235 0.1059 1] Handle MovementInput
  (Pawn|Input|AddMovementInput (Pawn|GetControlledPawn) (Math|Vector|ClampVectorSize (Math|Vector|MakeVector (.y ActionValue) (.x ActionValue) 0.0) 0.0 1.0) 1.0 false)
  ;[1 1 1] Enough time passed without any aim input to take over aiming based on movement
  (if (>= (- (Utilities|Time|GetTimeSeconds) (Variables|MouseAiming|GetLastAimInputTime)) (Variables|MouseAiming|GetMovementAimTimeDelay))
    ;[1 1 1] Disable & hide mouse aim
    (Variables|MouseAiming|SetUseMouseAim false)
    (bind _currentmouseaimtarget (Variables|MouseAiming|GetCurrentMouseAimTarget)
      (:then
        (Rendering|SetActorHiddenInGame _currentmouseaimtarget true)
        ;[1 1 1] Is there movement active?
        (if (> (Math|Vector|VectorLengthSquared _returnvalue_2) 0.0)
          (Pawn|SetControlRotation (Math|Rotator|MakeRotator (.roll _returnvalue_3) 0.0 (.yaw _returnvalue_3)))))
      (:else))))

(event EventBeginPlay
  (bind _returnvalue (PlayerController|LocalPlayerSubsystems|GetEnhancedInputLocalPlayerSubsystem))
  (Utilities|FlowControl|Sequence
    (:then_0
      ;[1 1 1] Enable default input mapping context
      (Utilities|IsValid _returnvalue
        (:Is%20Valid
          (Input|AddMappingContext _returnvalue "/Game/Input/IMC_Default.IMC_Default" 0 "(bIgnoreAllPressedKeysUntilRelease=True,bForceImmediately=False,bNotifyUserSettings=False)"))))
    (:then_1
      ;[1 1 1] Setup HUD
      (bind _returnvalue_2 (UserInterface|CreateWidget "/Game/Blueprints/BPW_MainMenu.BPW_MainMenu_C" self))
      (UserInterface|Viewport|AddtoViewport _returnvalue_2 0)
      ;[1 1 1] Pause game
      (Variables|Default|SetbShowMouseCursor true)
      (Game|SetGamePaused true))
    (:then_2
      (bind _outactors (Actor|GetAllActorsOfClass "/Game/Blueprints/BP_Interactable.BP_Interactable_C"))
      (Variables|Interactables|SetInteractables _outactors))))

(event EventTick
  (params (DeltaSeconds :type Float%20%28single-precision%29)))

(event Input|MouseEvents|Mouse2D
  (params (AxisValue :type Vector :default "0, 0, 0"))
  (bind (_hitresult _returnvalue) (Game|Player|GetHitResultUnderCursorbyChannel "TraceTypeQuery1" true))
  (bind _location (Collision|BreakHitResult _hitresult))
  ;[0.08235 0.1059 1] Mouse Aiming
  ;;[1 1 1] Detect Mouse Movement
  (Utilities|FlowControl|Sequence
    (:then_0
      ;;[1 0.4348 0] Detect if mouse aim input is big enough
      (if (> (Math|Vector|VectorLengthSquared AxisValue) 0.25)
        (Variables|MouseAiming|SetUseMouseAim true)
        (Variables|MouseAiming|SetLastAimInputTime (Utilities|Time|GetTimeSeconds))))
    (:then_1
      (if (Variables|MouseAiming|GetUseMouseAim)
        (Utilities|FlowControl|Sequence
          (:then_0
            ;;[1 1 1] Spawn MoueAimTarget & Store its Reference
            (Variables|MouseAiming|GetCurrentMouseAimTarget
              (:then)
              (:else
                (bind _returnvalue_2 (Game|SpawnActorfromClass "/Game/Blueprints/BP_MouseAimTarget.BP_MouseAimTarget_C" (Math|Transform|MakeTransform "0, 0, 0") "Undefined" "MultiplyWithRoot" 0 0))
                (Variables|MouseAiming|SetCurrentMouseAimTarget _returnvalue_2))))
          (:then_1
            ;;[1 1 1] Find position under mouse and rotate torwards that position
            (if _returnvalue
              (Pawn|SetControlRotation (Math|Rotator|MakeRotator 0.0 0.0 (.yaw (Math|Rotator|FindLookatRotation (Transformation|GetActorLocation (Pawn|GetControlledPawn)) _location))))
              ;;[1 1 1] Update MouseAimTarget position
              (bind _currentmouseaimtarget (Variables|MouseAiming|GetCurrentMouseAimTarget)
                (:then
                  (Rendering|SetActorHiddenInGame _currentmouseaimtarget false)
                  (Transformation|SetActorLocation _currentmouseaimtarget _location false false))
                (:else)))))))))

(fn ConstructionScript)

(fn EndMiniGame
  (params (MiniGameHUD :type User%20Widget%20Object%20Reference))
  (Widget|RemovefromParent MiniGameHUD))