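; BP_Interactable is an interactable actor that tracks player proximity and supports a cooldown-limited Interact event.
; Its Box overlap events cast to BP_PlayerCharacter and set or clear IsPlayerNearby.
; Interact, when CanInteract is true, prints a debug message, disables itself and starts a timer by function name that re-enables it after InteractionCooldown.
; Interact itself does not check IsPlayerNearby.
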(event OnComponentBeginOverlap(Box)
  (params (OverlappedComponent :type Primitive%20Component%20Object%20Reference) (OtherActor :type Actor%20Object%20Reference) (OtherComp :type Primitive%20Component%20Object%20Reference) (OtherBodyIndex :type Integer) (bFromSweep :type Boolean) (SweepResult :type Hit%20Result%20Structure%20%28by%20ref%29))
  (Utilities|Casting|CastToBP_PlayerCharacter OtherActor)
  (Variables|Default|SetIsPlayerNearby true))

(event OnComponentEndOverlap(Box)
  (params (OverlappedComponent :type Primitive%20Component%20Object%20Reference) (OtherActor :type Actor%20Object%20Reference) (OtherComp :type Primitive%20Component%20Object%20Reference) (OtherBodyIndex :type Integer))
  (Utilities|Casting|CastToBP_PlayerCharacter OtherActor)
  (Variables|Default|SetIsPlayerNearby false))

(event Custom|Interact
  (if (Variables|Default|GetCanInteract)
    (Variables|Default|SetCanInteract false)
    (Utilities|Time|SetTimerbyFunctionName 0 "ResetInteract" (Variables|Default|GetInteractionCooldown))
    (Development|PrintString "INTERACT!!")))

(event Custom|ResetInteract
  (Variables|Default|SetCanInteract true))

(event EventBeginPlay)

(event Collision|EventActorBeginOverlap
  (params (OtherActor :type Actor%20Object%20Reference)))

(event EventTick
  (params (DeltaSeconds :type Float%20%28single-precision%29)))

(fn ConstructionScript)