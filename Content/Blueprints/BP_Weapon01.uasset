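; Weapon Blueprint with two fire modes: repeating projectile shots and a continuous damage laser.
; Primary fire spawns a projectile and sound immediately, then repeats on a fire-rate timer.
; While secondary fire is held, Tick multi-traces from FireSocket, applying frame-scaled damage through the damageable interface on hit actors and their components.
; The laser pierces valid actors, stopping only at hits without one, which sets Niagara beam and light length.
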(event Custom|UpdateSecondaryLaserFire
  (bind _pointlight (Variables|Default|GetPointLight))
  (bind _firesocket (Variables|Default|GetFireSocket))
  (bind _returnvalue (Transformation|GetWorldLocation _firesocket))
  ;[1 1 1] Reset laser hit distance
  (Variables|SecondaryFire|SetLaserHitDistance (Variables|SecondaryFire|GetLaserDistance))
  ;[1 1 1] Line trace
  (bind _outhits (Class|KismetSystemLibrary|LineTraceMultiforObjects _returnvalue (+ _returnvalue (* (Math|Vector|GetForwardVector _firesocket) (Variables|SecondaryFire|GetLaserDistance))) (Utilities|Array|MakeArray "ObjectTypeQuery1" "ObjectTypeQuery3" "ObjectTypeQuery2") false 0 "None" true))
  (bind _array_element (Utilities|Array|ForEachLoopwithBreak _outhits :!label _label)
    (:LoopBody
      (Utilities|IsValid (.HitActor (Collision|BreakHitResult _array_element))
        (:Is%20Valid
          (CallFunction|ProcessLaserCollision (.HitActor (Collision|BreakHitResult _array_element)) (* (Variables|SecondaryFire|GetLaserDamagePerSecond) (Utilities|Time|GetWorldDeltaSeconds))))
        (:Is%20Not%20Valid
          (Variables|SecondaryFire|SetLaserHitDistance (.Distance (Collision|BreakHitResult _array_element)))
          (goto _label Break))))
    (:Completed
      ;[1 1 1] Adjust Beam target position
      (Effects|Components|ParticleSystem|SetVectorParameter (Variables|Default|GetBeam) "User.TargetPosition" (Math|Vector|MakeVector (Variables|SecondaryFire|GetLaserHitDistance) 0.0 0.0))
      ;[1 1 1] Adjust Beam light positioning & length
      (Class|PointLightComponent|SetSourceLength _pointlight (Variables|SecondaryFire|GetLaserHitDistance))
      (Transformation|SetRelativeLocation _pointlight (Math|Vector|MakeVector (/ (Variables|SecondaryFire|GetLaserHitDistance) 2.0) 0.0 0.0) false false))))

(event Custom|SpawnPrimaryProjectile
  ;[1 1 1] Handle Primary Fire
  (Audio|SpawnSoundAttached "/Game/Audio/466867__mikee63__blaster-shot-single-5.466867__mikee63__blaster-shot-single-5" (Variables|Default|GetWeaponMesh) "None" "0, 0, 0" "0, 0, 0" "KeepRelativeOffset" false 1.0 1.0 0.0 0 0)
  (Game|SpawnActorfromClass (Variables|PrimaryFire|GetPrimaryProjectileClass) (Transformation|GetWorldTransform (Variables|Default|GetFireSocket)) "Undefined" "MultiplyWithRoot" 0 0))

(event EventBeginPlay
  (|CallParentFunction)
  ;[1 1 1] Hide Beam on Start
  (Development|SetHiddeninGame (Variables|Default|GetBeam) true true))

(event Collision|EventActorBeginOverlap
  (params (OtherActor :type Actor%20Object%20Reference))
  (|CallParentFunction OtherActor) ; This node is disabled and will not be called.\nDrag off pins to build functionality.
)

(event EventTick
  (params (DeltaSeconds :type Float%20%28single-precision%29))
  (|CallParentFunction DeltaSeconds)
  (if (Variables|SecondaryFire|GetEnableSecondaryFireLaser)
    (CallFunction|UpdateSecondaryLaserFire)))

(event EventFirePrimary
  (params (IsStart :type Boolean))
  ;[1 1 1] Handle Primary Fire
  (|CallParentFunction IsStart)
  (if IsStart
    (Utilities|FlowControl|DoOnce false :!label _label
      (:Completed
        ;;[1 1 1] Instant first shoot
        (CallFunction|SpawnPrimaryProjectile)
        (Utilities|Time|SetTimerbyEvent (delegate Custom|SpawnPrimaryProjectile) (/ 1.0 (Variables|PrimaryFire|GetPrimaryFireRate)) true)))
    (else
      (Utilities|Time|ClearTimerbyFunctionName 0 "SpawnPrimaryProjectile")
      (goto _label Reset))))

(event EventFireSecondary
  (params (IsStart :type Boolean))
  ;[1 1 1] Handle Secondary Fire Input
  (|CallParentFunction IsStart)
  (bind _output_get (Variables|SecondaryFire|SetEnableSecondaryFireLaser IsStart))
  (Development|SetHiddeninGame (Variables|Default|GetBeam) (not _output_get) true))

(fn ConstructionScript
  (|CallParentFunction))

(fn ProcessLaserCollision
  (params (OtherActor :type Actor%20Object%20Reference) (DamageAmount :type Float%20%28double-precision%29))
  (bind _returnvalue (Class|Actor|GetComponentsbyInterface OtherActor "/Script/Unreal101.DamageableInterface"))
  ;[1 1 1] Check if we actually hit actor
  (Utilities|IsValid OtherActor
    (:Is%20Valid
      ;[1 1 1] Check if target doesn't have matching ignore tag
      (if (not (Actor|ActorHasTag (Variables|SecondaryFire|GetLaserIgnoreTag)))
        (Utilities|FlowControl|Sequence
          (:then_0
            ;[1 1 1] BPI_Damagable on hit actor
            (if (Utilities|DoesObjectImplementInterface OtherActor "/Script/Unreal101.DamageableInterface")
              (Class|DamageableInterface|DoDamage(Message) OtherActor DamageAmount)))
          (:then_1
            ;[1 1 1] Get all component that implement the BPI_Damagable interface & DoDagame
            (Utilities|IsValid OtherActor
              (:Is%20Valid
                (bind _index (Utilities|FlowControl|ForLoopwithBreak 0 (- (Utilities|Array|Length _returnvalue) 1) :!label _label)
                  (:LoopBody
                    (Class|DamageableInterface|DoDamage(Message) (Utilities|Array|Get(acopy) _returnvalue _index) DamageAmount)
                    (Utilities|IsValid OtherActor
                      (:Is%20Not%20Valid
                        (goto _label Break)))))))))))))