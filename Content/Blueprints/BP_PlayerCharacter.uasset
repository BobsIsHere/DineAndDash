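; Player character Blueprint that holds three condiment amounts: salt, cheese and herb.
; Tick keeps each amount from dropping below zero, and a custom refill event per condiment restores it to the shared maximum.
; BeginPlay attaches the Slick_Victory_Loop sound to the character mesh.
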(event Custom|RefillSaltCondiment
  ;[1 1 1] Condiments Refill Events
  (Variables|Condiments|SetSaltAmount (+ (- (Variables|Condiments|GetMaxCondimentAmount) (Variables|Condiments|GetSaltAmount)) (Variables|Condiments|GetSaltAmount))))

(event Custom|RefillCheeseCondiment
  ;[1 1 1] Condiments Refill Events
  (Variables|Condiments|SetCheeseAmount (+ (- (Variables|Condiments|GetMaxCondimentAmount) (Variables|Condiments|GetCheeseAmount)) (Variables|Condiments|GetCheeseAmount))))

(event Custom|RefillHerbCondiment
  ;[1 1 1] Condiments Refill Events
  (Variables|Condiments|SetHerbAmount (+ (- (Variables|Condiments|GetMaxCondimentAmount) (Variables|Condiments|GetHerbAmount)) (Variables|Condiments|GetHerbAmount))))

(event EventBeginPlay
  (|CallParentFunction)
  (Audio|SpawnSoundAttached "/Game/Sounds/Slick_Victory_Loop.Slick_Victory_Loop" (Variables|Character|GetMesh) "None" "0, 0, 0" "0, 0, 0" "KeepRelativeOffset" false 0.1 1.0 0.0 0 0))

(event Collision|EventActorBeginOverlap
  (params (OtherActor :type Actor%20Object%20Reference))
  (|CallParentFunction OtherActor) ; This node is disabled and will not be called.\nDrag off pins to build functionality.
)

(event EventTick
  (params (DeltaSeconds :type Float%20%28single-precision%29))
  (|CallParentFunction DeltaSeconds)
  ;[1 1 1] No negative Condiment amounts
  (if (<= (Variables|Condiments|GetSaltAmount) 0)
    (Variables|Condiments|SetSaltAmount 0))
  (if (<= (Variables|Condiments|GetCheeseAmount) 0)
    (Variables|Condiments|SetCheeseAmount 0))
  (if (<= (Variables|Condiments|GetHerbAmount) 0)
    (Variables|Condiments|SetHerbAmount 0)))

(fn ConstructionScript
  (|CallParentFunction))