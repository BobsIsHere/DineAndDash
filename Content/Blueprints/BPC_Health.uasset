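; Health component that tracks current health against a maximum and signals when it is depleted.
; BeginPlay resets health to max, and DoDamage subtracts an amount, clamped between zero and max, then returns whether health is depleted.
; It fires OnDeath only when that damage lowered health to zero, so hits on an already dead owner do not fire it again.
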(event Custom|ResetHealth
  (Variables|Health|SetCurrentHealth (Variables|Health|GetMaxHealth)))

(event EventBeginPlay
  (CallFunction|ResetHealth))

(event EventTick
  (params (DeltaSeconds :type Float%20%28single-precision%29)))

(fn GetHealthPercentage
  (return (/ (Variables|Health|GetCurrentHealth) (Variables|Health|GetMaxHealth))))

(fn IsDead
  (return (<= (CallFunction|GetHealthPercentage) 0.0)))

(fn DoDamage
  (params (Amount :type Float%20%28double-precision%29))
  (bind _isdead (CallFunction|IsDead))
  (LocalVariables|SetOriginalHealth (Variables|Health|GetCurrentHealth))
  ;[1 1 1] Store adjusted health value
  (bind _output_get (Variables|Health|SetCurrentHealth (Math|Float|Clamp(Float) (- (Variables|Health|GetCurrentHealth) Amount) 0.0 (Variables|Health|GetMaxHealth))))
  ;[1 1 1] Did this DoDamage cause the health to change and drop below 0
  (if (and _isdead (> (LocalVariables|GetOriginalHealth) _output_get))
    (Default|CallOnDeath))
  (return _isdead))

(fn DoDamage
  (params (amount :type Float%20%28single-precision%29))
  (bind _isdead (CallFunction|IsDead))
  (LocalVariables|SetOriginalHealth (Variables|Health|GetCurrentHealth))
  ;[1 1 1] Store adjusted health value
  (bind _output_get (Variables|Health|SetCurrentHealth (Math|Float|Clamp(Float) (- (Variables|Health|GetCurrentHealth) amount) 0.0 (Variables|Health|GetMaxHealth))))
  ;[1 1 1] Did this DoDamage cause the health to change and drop below 0
  (if (and _isdead (> (LocalVariables|GetOriginalHealth) _output_get))
    (Default|CallOnDeath))
  (return _isdead))