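; Enemy spawner that spawns a BP_EnemyCharacter with AI when its Spawn event is called.
; It caps live enemies using MaxAmountOfActiveEnemiesActors from BP_MyGameMode, defaulting to zero if the cast fails.
; Location is either a random point in SpawnVolume or the root position, per UseSpawnVolume.
; IsSpawning blocks repeat calls until a SpawnInterval timer resets it, but stays set when the cap check fails because no timer starts.
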(event Custom|Spawn
  (bind _returnvalue (Game|GetGameMode))
  (bind _spawnvolume (Variables|Default|GetSpawnVolume))
  (bind (_asbp_my_game_mode _bsuccess) (Utilities|Casting|CastToBP_MyGameMode _returnvalue))
  (if (not (Variables|Default|GetIsSpawning))
    (Variables|Default|SetIsSpawning true)
    ;[1 1 1] Limit the number of spawns
    (bind _outactors (Actor|GetAllActorsOfClass "/Game/Blueprints/BP_EnemyCharacter.BP_EnemyCharacter_C"))
    (if (not (> (Utilities|Array|Length _outactors) (Math|Integer|SelectInt (Variables|/Game/Blueprints/BP_MyGameMode.BP_MyGameMode_C|GetMaxAmountOfActiveEnemiesActors _asbp_my_game_mode) 0 _bsuccess)))
      ;[1 1 1] Select a spawn location
      (AI|SpawnAIFromClass "/Game/Blueprints/BP_EnemyCharacter.BP_EnemyCharacter_C" 0 (Math|Vector|SelectVector (Math|Random|RandomPointinBoundingBox (Transformation|GetWorldLocation _spawnvolume) (Components|Box|GetScaledBoxExtent _spawnvolume)) (Transformation|GetWorldLocation (Variables|Default|GetDefaultSceneRoot)) (Variables|Default|GetUseSpawnVolume)) (Transformation|GetWorldRotation (Variables|Default|GetDefaultSceneRoot)) false 0)
      (Utilities|Time|SetTimerbyFunctionName 0 "ResetRespawn" (Variables|Default|GetSpawnInterval)))))

(event Custom|ResetRespawn
  (Variables|Default|SetIsSpawning false))

(event EventBeginPlay)

(event Collision|EventActorBeginOverlap
  (params (OtherActor :type Actor%20Object%20Reference)))

(event EventTick
  (params (DeltaSeconds :type Float%20%28single-precision%29)))

(fn ConstructionScript)