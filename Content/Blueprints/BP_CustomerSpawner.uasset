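; Customer spawner that creates AI customer characters while tables are free, using a longer interval in tutorial mode.
; Spawn locks on the first free table, then spawns at the root or a random volume point if the game mode's active-customer cap allows.
; A timer clears the lock after a successful spawn; a blocked or failed attempt leaves it set.
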(event Custom|Spawn
  (bind _returnvalue (Game|GetGameMode))
  (bind _spawnvolume (Variables|Default|GetSpawnVolume))
  (bind (_asbp_base_game_mode _bsuccess) (Utilities|Casting|CastToBP_BaseGameMode _returnvalue))
  (bind _outactors (Actor|GetAllActorsOfClass "/Game/Blueprints/Interactables/BPI_Table.BPI_Table_C"))
  (for _array_element _outactors
    (if (not (Variables|/Game/Blueprints/Interactables/BPI_Table.BPI_Table_C|GetIsTableOccupied _array_element))
      (if (not (Variables|Default|GetIsSpawning))
        (Variables|Default|SetIsSpawning true)
        ;[1 1 1] Limit the number of spawns
        (bind _outactors_2 (Actor|GetAllActorsOfClass "/Game/Blueprints/BP_CustomerCharacter.BP_CustomerCharacter_C"))
        (if (not (> (Utilities|Array|Length _outactors_2) (Math|Integer|SelectInt (Variables|/Game/Blueprints/BP_BaseGameMode.BP_BaseGameMode_C|GetMaxAmountOfActiveCustomers _asbp_base_game_mode) 0 _bsuccess)))
          ;[1 1 1] Select a spawn location
          (bind _returnvalue_2 (AI|SpawnAIFromClass "/Game/Blueprints/BP_CustomerCharacter.BP_CustomerCharacter_C" 0 (Math|Vector|SelectVector (Math|Random|RandomPointinBoundingBox (Transformation|GetWorldLocation _spawnvolume) (Components|Box|GetScaledBoxExtent _spawnvolume)) (Transformation|GetWorldLocation (Variables|Default|GetDefaultSceneRoot)) (Variables|Default|GetUseSpawnVolume)) (Transformation|GetWorldRotation (Variables|Default|GetDefaultSceneRoot)) false 0))
          (Utilities|IsValid _returnvalue_2
            (:Is%20Valid
              (Utilities|Time|SetTimerbyFunctionName 0 "ResetRespawn" (Variables|Default|GetSpawnInterval)))))))))

(event Custom|ResetRespawn
  (Variables|Default|SetIsSpawning false))

(event EventBeginPlay
  ;[1 1 1] Set Spawn Interval Based on Game Mode
  (Utilities|Casting|CastToBP_TutorialGameMode (Game|GetGameMode)
    (:then
      (Variables|Default|SetSpawnInterval 8.0))
    (:CastFailed
      (Variables|Default|SetSpawnInterval 4.0))))

(fn ConstructionScript)