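; Enemy character that damages an overlapping player on a looping timer and awards score through BP_MyGameMode on death.
; The timer starts on player overlap and clears when that player leaves or the enemy dies.
; Construction creates dynamic materials for body color and a health indicator, which updates every tick from a color curve with a yellow fallback.
; Death disables movement and collision, plays a sound and destroys the actor after a delay.
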(event OnDeath(BPC_Health)
  ;[1 1 1] Death
  (Utilities|FlowControl|Sequence
    (:then_0
      ;;[1 1 1] Increment Score
      (bind _asbp_my_game_mode (Utilities|Casting|CastToBP_MyGameMode (Game|GetGameMode)))
      (Default|IncrementScore _asbp_my_game_mode (Variables|Default|GetScoreAmount)))
    (:then_1
      (Pawn|Components|CharacterMovement|DisableMovement (Variables|Character|GetCharacterMovement))
      (Utilities|Time|ClearTimerbyFunctionName 0 "DamageCurrentPlayerTarget")
      (Collision|SetCollisionEnabled (Variables|Default|GetDamageVolume) "NoCollision")
      (Collision|SetCollisionEnabled (Variables|Default|GetCapsuleComponent) "NoCollision")
      (Audio|SpawnSoundAttached "/Game/Audio/DeathVocalisation.DeathVocalisation" (Variables|Character|GetMesh) "None" "0, 0, 0" "0, 0, 0" "KeepRelativeOffset" false 1.0 1.0 0.0 0 0)
      (Utilities|FlowControl|Delay 3.0)
      (Actor|DestroyActor))))

(event Custom|DamageCurrentPlayerTarget
  (bind _currentplayertarget (Variables|Damage|GetCurrentPlayerTarget))
  (Utilities|IsValid _currentplayertarget
    (:Is%20Valid
      (Class|DamageableInterface|DoDamage (Variables|/Game/Blueprints/BP_BaseCharacter.BP_BaseCharacter_C|GetBPC_Health _currentplayertarget) (Variables|Damage|GetDamageAmount)))))

(event EventBeginPlay
  (|CallParentFunction) ; This node is disabled and will not be called.\nDrag off pins to build functionality.
)

(event Collision|EventActorBeginOverlap
  (params (OtherActor :type Actor%20Object%20Reference))
  ;[1 1 1] Detect Player Collision
  (|CallParentFunction OtherActor)
  (bind _asbp_player_character (Utilities|Casting|CastToBP_PlayerCharacter OtherActor))
  (Variables|Damage|SetCurrentPlayerTarget _asbp_player_character)
  (Utilities|Time|SetTimerbyEvent (delegate Custom|DamageCurrentPlayerTarget) (Variables|Default|GetAttackInterval) true))

(event EventTick
  (params (DeltaSeconds :type Float%20%28single-precision%29))
  (|CallParentFunction DeltaSeconds)
  (CallFunction|UpdateHealthIndicator))

(event Collision|EventActorEndOverlap
  (params (OtherActor :type Actor%20Object%20Reference))
  ;[1 1 1] Detect Player Collision loss
  (if (== OtherActor (Variables|Damage|GetCurrentPlayerTarget))
    (Utilities|Time|ClearTimerbyFunctionName 0 "DamageCurrentPlayerTarget")))

(fn ConstructionScript
  (bind _mesh (Variables|Character|GetMesh))
  (|CallParentFunction)
  (bind _returnvalue (Rendering|Material|CreateDynamicMaterialInstance _mesh 0 0 "None" :!class /Script/Engine.PrimitiveComponent))
  (bind _output_get (Variables|Enemy|SetBodyMaterialInstance _returnvalue))
  (Rendering|Material|SetVectorParameterValue _output_get "BodyColor" (Variables|Enemy|GetEnemyColor) :!class /Script/Engine.MaterialInstanceDynamic)
  (bind _returnvalue_2 (Rendering|Material|CreateDynamicMaterialInstance _mesh 1 0 "None" :!class /Script/Engine.PrimitiveComponent))
  (Variables|Enemy|SetHealthMaterialInstance _returnvalue_2)
  (CallFunction|UpdateHealthIndicator))

(fn UpdateHealthIndicator
  (bind _healthcurve (Variables|Enemy|GetHealthCurve))
  (bind _healthmaterialinstance (Variables|Enemy|GetHealthMaterialInstance)
    (:then
      (Rendering|Material|SetVectorParameterValue _healthmaterialinstance "Color" (Math|Color|SelectColor (Math|Curves|GetLinearColorValue _healthcurve (Default|GetHealthPercentage (Variables|Default|GetBPC_Health))) "(R=1.000000,G=0.988338,B=0.000000,A=1.000000)" (Utilities|IsValid _healthcurve)) :!class /Script/Engine.MaterialInstanceDynamic))
    (:else)))